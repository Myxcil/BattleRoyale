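; BP_Plane is a C-130J transport plane actor in the BR content that carries a player spawn point.
; The construction script registers its PlayerSpawnPoint through SetPlayerSpawn.
; On BeginPlay it casts the mesh's anim instance to the C130J animation Blueprint and sets a fixed pose: propellers spinning, wheel retract values at full and ramp open.
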(event EventBeginPlay
  (bind _asbpa_west_transport_c130j (Utilities|Casting|CastToBPA_West_Transport_C130J (Components|SkeletalMesh|GetAnimInstance (Variables|Default|GetPlaneMesh))))
  (bind _output_get (Variables|Default|SetAnimInstance _asbpa_west_transport_c130j))
  (Variables|/Game/VigilanteContent/Vehicles/West_Transport_C130J/BPA_West_Transport_C130J.BPA_West_Transport_C130J_C|SetPropellerSpeed _output_get 5e+02)
  (Variables|/Game/VigilanteContent/Vehicles/West_Transport_C130J/BPA_West_Transport_C130J.BPA_West_Transport_C130J_C|SetFrontWheelRetract _output_get 1.0)
  (Variables|/Game/VigilanteContent/Vehicles/West_Transport_C130J/BPA_West_Transport_C130J.BPA_West_Transport_C130J_C|SetRearWheelLRetract _output_get 1.0)
  (Variables|/Game/VigilanteContent/Vehicles/West_Transport_C130J/BPA_West_Transport_C130J.BPA_West_Transport_C130J_C|SetRearWheelRRetract _output_get 1.0)
  (Variables|/Game/VigilanteContent/Vehicles/West_Transport_C130J/BPA_West_Transport_C130J.BPA_West_Transport_C130J_C|SetRampOpen _output_get 1.0))

(fn ConstructionScript
  (Class|BRPlane|SetPlayerSpawn (Variables|Default|GetPlayerSpawnPoint)))